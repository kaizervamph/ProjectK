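; BP_CornerFixer is a corner filler piece for the building system that avoids showing duplicates where fixers overlap.
; On construction, CheckCollision queries the Box for other visible BP_CornerFixer actors and shows Cube6 only if none are found.
; Two events apply exterior and interior materials to separate Cube6 slots.
; The logic copying materials from a parent BP_EBS_Building_Wall is disconnected, as is BeginPlay.
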(event `self.ReceiveBeginPlay`)

(event `SetExteriorMaterial`
  (params (Material :type "MaterialInterface Object Reference"))
  (bind _cube6 (`self.Cube6`))
  (`PrimitiveComponent.SetMaterial` _cube6 0 Material)
  (`PrimitiveComponent.SetMaterial` _cube6 2 Material)
  (`PrimitiveComponent.SetMaterial` _cube6 4 Material))

(event `SetInteriorMaterial`
  (params (Material :type "MaterialInterface Object Reference"))
  (`PrimitiveComponent.SetMaterial` (`self.Cube6`) 3 Material))

(fn `CheckCollision`
  (returns (Success :type Boolean))
  (bind _builds (`self.GetOverlapedBuilds` (`self.Box`)))
  (`SceneComponent.SetVisibility` (`self.Cube6`) (<= (`KismetArrayLibrary.Array_Length` _builds) 0) false)
  (return true))

(fn `GetOverlapedBuilds`
  (params (Component :type "PrimitiveComponent Object Reference"))
  (returns (Builds :type "Array of Actor Object Reference"))
  (locals (Temp :type "Array of Actor Object Reference"))
  (bind _outactors (`KismetSystemLibrary.ComponentOverlapActors` Component (`self.GetTransform`) (`|MakeArray` "ObjectTypeQuery1" "ObjectTypeQuery2" :!type "EObjectTypeQuery Enum") null (`|MakeArray` self :!type "Actor Object Reference")))
  (for _array_element _outactors
    (bind _asbp_corner_fixer (cast `/Game/BurdelKing/BP_CornerFixer` _array_element))
    (if (`self.IsVisible?` _asbp_corner_fixer)
      (`KismetArrayLibrary.Array_Add` (`local.Temp`) _asbp_corner_fixer)))
  (return (`local.Temp`)))

(fn `IsVisible?`
  (returns (Visibility :type Boolean))
  (return (`SceneComponent.bVisible` (`self.Cube6`))))

(fn `UserConstructionScript`
  (`self.CheckCollision`))