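; BP_PedestrianBase is the base pedestrian that either walks by or heads to the brothel (Burdel), chosen at random on BeginPlay.
; It randomizes body-shape morph targets, shows its indicator sphere only for walk-bys, then tells its AIC_Pedestrian controller to call NextPoint or GoToBurdel.
; Cursor hover toggles the mesh's custom depth rendering, and ChangeIndicator switches the sphere between green and red materials based on its Consume flag.
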(event `self.ReceiveBeginPlay`
  (`self.RandomShapes`)
  (bind _output_get (set `self.Walkby` (`KismetMathLibrary.RandomBool`)))
  (`SceneComponent.SetVisibility` (`self.Sphere`) _output_get false)
  (bind _asaic_pedestrian (cast `/Game/BurdelKing/Pedestrians/AIC_Pedestrian` (`AIBlueprintHelperLibrary.GetAIController` self)))
  (if _output_get
    (`/Game/BurdelKing/Pedestrians/AIC_Pedestrian.NextPoint` _asaic_pedestrian)
    (else
      (`/Game/BurdelKing/Pedestrians/AIC_Pedestrian.GoToBurdel` _asaic_pedestrian))))

(event `RandomShapes`
  (bind _mesh (`self.Mesh`))
  (`|ExecutionSequence`
    (:`then_0`
      (`SkeletalMeshComponent.SetMorphTarget` _mesh "BD Figure Skinny" (`KismetMathLibrary.RandomFloatInRange` -1.0 1.0) true))
    (:`then_1`
      (`SkeletalMeshComponent.SetMorphTarget` _mesh "BD Figure Skinny Breasts" (`KismetMathLibrary.RandomFloatInRange` -1.0 1.0) true))
    (:`then_2`
      (`SkeletalMeshComponent.SetMorphTarget` _mesh "BD Figure Pear" (`KismetMathLibrary.RandomFloatInRange` -1.0 1.0) true))))

(event `self.Mesh.OnBeginCursorOver`
  (params (TouchedComponent :type "PrimitiveComponent Object Reference"))
  (`PrimitiveComponent.SetRenderCustomDepth` (`self.Mesh`) true))

(event `self.Mesh.OnEndCursorOver`
  (params (TouchedComponent :type "PrimitiveComponent Object Reference"))
  (`PrimitiveComponent.SetRenderCustomDepth` (`self.Mesh`) false))

(event `ChangeIndicator`
  (params (Consume :type Boolean))
  (`PrimitiveComponent.SetMaterial` (`self.Sphere`) 0 (select `bool` Consume :`false` "/AnimationSharing/AnimSharingRed.AnimSharingRed" :`true` "/AnimationSharing/AnimSharingGreen.AnimSharingGreen" :!type "MaterialInterface Object Reference")))

(fn `UserConstructionScript`)