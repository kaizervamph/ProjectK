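; BP_PedestrianSpawn is a spawner actor that keeps adding random pedestrians to the world under a population limit.
; On BeginPlay it starts a looping timer with an interval picked once between random bounds.
; Each tick of that timer counts all BP_PedestrianBase actors and, if the count is at or below Limit, spawns a random class from PederstiansList at its location.
; It then enables movement logic on the new pedestrian's AIC_Pedestrian controller.
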(event `self.ReceiveBeginPlay`
  (`KismetSystemLibrary.K2_SetTimerDelegate` (delegate `Spawn`) (`KismetMathLibrary.RandomFloatInRange` 5.0 10.0) true))

(event `Spawn`
  (bind _outactors (`GameplayStatics.GetAllActorsOfClass` "/Game/BurdelKing/Pedestrians/BP_PedestrianBase.BP_PedestrianBase_C"))
  (if (<= (`KismetArrayLibrary.Array_Length` _outactors) (`self.Limit`))
    (bind _returnvalue (`|SpawnActorFromClass` (`KismetArrayLibrary.Array_Random` (`self.PederstiansList`)) (`KismetMathLibrary.Conv_VectorToTransform` (`self.K2_GetActorLocation`)) "AlwaysSpawn" "OverrideRootScale" null null))
    (bind _asaic_pedestrian (cast `/Game/BurdelKing/Pedestrians/AIC_Pedestrian` (`AIBlueprintHelperLibrary.GetAIController` _returnvalue)))
    (`/Game/BurdelKing/Pedestrians/AIC_Pedestrian.EnableMovementLogic` _asaic_pedestrian)))

(fn `UserConstructionScript`)