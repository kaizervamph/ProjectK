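; Doll actor that renders face portraits of procedurally generated characters and also backs the CharacterCreator level's morph-target UI.
; A looping timer builds the first queued character's meshes, captures it with a self-only SceneCapture2D, and converts it to a texture and bytes.
; Results go to BP_GenerateCharactersActor until its Amount is reached.
; A DoOnce gates each capture until ResetCapture removes the finished entry and reopens it.
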(event `self.ReceiveBeginPlay`
  (`KismetArrayLibrary.Array_Add` (`SceneCaptureComponent.ShowOnlyActors` (`self.SceneCaptureComponent2D`)) self)
  (bind _returnvalue (`GameplayStatics.GetCurrentLevelName` true))
  (if (`KismetStringLibrary.EqualEqual_StrStr` _returnvalue "CharacterCreator")
    (`self.CharacterCreatorLogic`)))

(event `CharacterCreatorLogic`
  (bind _returnvalue (`|CreateWidget` "/Game/CharacterCreator/WBP_CharacterCreator.WBP_CharacterCreator_C"))
  (set `self.CC_Ref` _returnvalue)
  (`UserWidget.AddToViewport` _returnvalue 0)
  (`/Game/ProceduralGeneration/FL_ProceduralGeneration.SetBodyMesh` (make `/Game/ProceduralGeneration/ProceduralCharacterStruct` :`BodyMesh` "/Game/Assets/SK_Female_01.SK_Female_01" :`AnimationBP` "/Game/Assets/ABP_Female_01.ABP_Female_01_C") (`self.BodyMesh`))
  (bind _cc_ref (`self.CC_Ref`)
    (:`then`
      (`/Game/CharacterCreator/WBP_CharacterCreator.LoadMorphoTarget` _cc_ref (`SkeletalMesh.K2_GetAllMorphTargetNames` (`SkinnedMeshComponent.SkeletalMesh` (`self.BodyMesh`)))))
    (:`else`)))

(event `GenerateRendersFromAttributes`
  (params (Attributes :type "Array of /Game/ProceduralGeneration/ProceduralCharacterStruct Structure"))
  (bind _output (`|GetArrayItem` (`self.CharactersToGenerate`)))
  (set `self.CharactersToGenerate` Attributes)
  (set `self.RendersAmount` 0)
  (`|ExecutionSequence`
    (:`then_0`
      (`KismetSystemLibrary.K2_SetTimerDelegate` (delegate `Renders`) 0.1 true))
    (:`then_1`
      (bind _generatoractor (`self.GetGeneratorActor` :!label _label))
      (if (!= (`/Game/ProceduralGeneration/BP_GenerateCharactersActor.Amount` _generatoractor) (`self.RendersAmount`))
        (`/Engine/EditorBlueprintResources/StandardMacros.DoOnce` false :!label _label_2
          (:`Completed`
            (bind _returnvalue (`AddComponent|NODE_AddSkeletalMeshComponent-1`))
            (bind _returnvalue_2 (`AddComponent|NODE_AddSkeletalMeshComponent-2`))
            (`/Game/ProceduralGeneration/FL_ProceduralGeneration.ConfigCharacterMeshes` self (`self.BodyMesh`) (`self.Meshes`) _output (`|MakeArray` _returnvalue) _returnvalue_2)
            (`KismetSystemLibrary.Delay` 0.1)
            (bind (_sizex _sizey _bytes _texture) (`self.CaptureRender`))
            (bind _generatoractor_2 (`self.GetGeneratorActor`))
            (bind _structout (setmembers `/Game/ProceduralGeneration/ProceduralCharacterStruct` :`StructRef` _output :`FaceRender` _texture :`FaceRenderBytes` _bytes :`RenderSize` (make `Int32Range` (make `Int32RangeBound` "Exclusive" _sizex) (make `Int32RangeBound` "Exclusive" _sizey))))
            (`/Game/ProceduralGeneration/BP_GenerateCharactersActor.AddGeneratedCharacter` _generatoractor_2 _structout self)
            (`/Engine/EditorBlueprintResources/StandardMacros.IncrementInt` (`self.RendersAmount`))))
        (else
          (`KismetSystemLibrary.K2_ClearTimer` self "Renders"))))))

(event `Renders`
  (goto _label))

(event `ResetCapture`
  (`KismetArrayLibrary.Array_Remove` (`self.CharactersToGenerate`))
  (goto _label_2 :!via `Reset`))

(fn `CaptureRender`
  (returns (SizeX :type Integer) (SizeY :type Integer) (Bytes :type "Array of Byte") (Texture :type "Texture2D Object Reference"))
  (locals (RT :type "TextureRenderTarget2D Object Reference"))
  (bind _scenecapturecomponent2d (`self.SceneCaptureComponent2D`))
  (bind _texturetarget (`SceneCaptureComponent2D.TextureTarget` _scenecapturecomponent2d))
  (bind _sizex (`TextureRenderTarget2D.SizeX` _texturetarget))
  (bind _sizey (`TextureRenderTarget2D.SizeY` _texturetarget))
  (`SceneCaptureComponent2D.CaptureScene` _scenecapturecomponent2d)
  (bind _outimagedata (`self.CaptureSceneTexture` (`self.SceneCaptureComponent2D`)))
  (bind _returnvalue (`self.CreateTextureFromImageData` _outimagedata _sizex _sizey))
  (return _sizex _sizey _outimagedata _returnvalue))

(fn `GetGeneratorActor`
  (returns (GeneratorActor :type "/Game/ProceduralGeneration/BP_GenerateCharactersActor Object Reference"))
  (bind _outactors (`GameplayStatics.GetAllActorsOfClass` "/Game/ProceduralGeneration/BP_GenerateCharactersActor.BP_GenerateCharactersActor_C"))
  (return (`|GetArrayItem` _outactors)))

(fn `UserConstructionScript`)