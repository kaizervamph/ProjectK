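; Base employee character that assembles its body and clothing meshes, then runs an AI work routine in the building.
; Chained AIMoveTo calls retry on failure, leading from a random foundation via a locker room to an activity with free capacity.
; When the job montage completes, it leaves that activity and picks another.
; It also captures a face render texture through BP_DollRenderActor for its UI slot and can randomise skin colour via dynamic materials.
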(event `self.ReceiveBeginPlay`
  (bind _returnvalue (`AddComponent|NODE_AddSkeletalMeshComponent-1`))
  (`/Game/ProceduralGeneration/FL_ProceduralGeneration.ConfigCharacterMeshes` self (`self.Mesh`) (`self.Meshes`) (`self.CharacterInfo`) (`|MakeArray` _returnvalue))
  (`self.GoToWork`))

(event `GoToWork`
  (bind _location (`self.GetWorkPlace`))
  (`|AIMoveTo` self _location null
    (:`OnSuccess`
      (`self.GoToLockerRoom`))
    (:`OnFail`
      (`self.GoToWork`))))

(event `CaptureRender`
  (`KismetSystemLibrary.Delay` 0.1)
  (bind _outactors (`GameplayStatics.GetAllActorsOfClass` "/Game/BurdelKing/BP_DollRenderActor.BP_DollRenderActor_C"))
  (if (`KismetArrayLibrary.Array_IsValidIndex` _outactors)
    (`self.GetChildMesh`)
    (bind _output (`|GetArrayItem` _outactors))
    (bind (_sizex _sizey) (`/Game/BurdelKing/BP_DollRenderActor.CaptureRender` _output))
    (bind (_outimagedata _returnvalue) (`CPP_StrippClubActor.CaptureSceneTexture` _output (`self.SceneCaptureComponent2D`)))
    (if _returnvalue
      (bind _output_get (set `self.FaceRenderData` (make `/Game/BurdelKing/RendersStruct` _outimagedata _sizex _sizey)))
      (bind (_imagendata _sizex_2 _sizey_2) (break `/Game/BurdelKing/RendersStruct` _output_get))
      (bind _returnvalue_2 (`CPP_StrippClubActor.CreateTextureFromImageData` _output _imagendata _sizex_2 _sizey_2 "PF_B8G8R8A8"))
      (set `self.FaceRenderTexture` _returnvalue_2)
      (bind (_find _widget) (`self.GetOwnEmployeesSlot`))
      (if _find
        (`/Game/BurdelKing/WBP_OwnEmployeSlot.HiddenLoader` _widget))
      (else
        (`KismetSystemLibrary.PrintString` "FaceRender FAIL" true true (struct :`R` 1.0 :`G` 0.043376 :`A` 1.0) 22.0)))))

(event `ChangeSkinColor`
  (bind _mesh (`self.Mesh`))
  (for (_array_element _array_index) (`MeshComponent.GetMaterials` _mesh)
    (bind _returnvalue (`PrimitiveComponent.CreateDynamicMaterialInstance` _mesh _array_index _array_element "None"))
    (bind _output_get (set `self.SkinColor` (`KismetArrayLibrary.Array_Random` (`|MakeArray` (struct :`R` 1.0 :`A` 1.0) (struct :`G` 1.0 :`A` 1.0) (struct :`B` 1.0 :`A` 1.0) :!type "LinearColor Structure"))))
    (`MaterialInstanceDynamic.SetVectorParameterValue` _returnvalue "SkinColor" _output_get)
    (`PrimitiveComponent.SetMaterial` _mesh _array_index _returnvalue))
  (`KismetSystemLibrary.PrintString` (`KismetStringLibrary.Concat_StrStr` "SkinColor=" (`KismetStringLibrary.Conv_ColorToString` (`self.SkinColor`))) true true (struct :`G` 0.66 :`B` 1.0 :`A` 1.0) 10.0))

(event `GoToLockerRoom`
  (bind _location (`self.GetLockerRoom`))
  (`|AIMoveTo` self _location null
    (:`OnSuccess`
      (`self.SetJobCloth`))
    (:`OnFail`
      (`self.GoToLockerRoom`))))

(event `SetJobCloth`
  (`self.GoToJobActivity`))

(event `GoToJobActivity`
  (bind _activity (`self.GetJobActivity`))
  (bind _output_get (set `self.SelectedActivity` _activity))
  (`|AIMoveTo` self (`self.K2_GetActorLocation` _output_get) null (`/Game/EasyBuildingSystem/Blueprints/BuildingObjects/Placeable/Poles/BP_EBS_Building_Activity.RangeAcceptable` (`self.SelectedActivity`))
    (:`OnSuccess`
      (bind _selectedactivity (`self.SelectedActivity`)
        (:`then`
          (`/Game/EasyBuildingSystem/Blueprints/BuildingObjects/Placeable/Poles/BP_EBS_Building_Activity.TryJob` _selectedactivity self))
        (:`else`)))
    (:`OnFail`
      (`self.GoToJobActivity`))))

(event `PlayJobMontage`
  (params (Montage :type "AnimMontage Object Reference") (ActivityActor :type "/Game/EasyBuildingSystem/Blueprints/BuildingObjects/Placeable/Poles/BP_EBS_Building_Activity Object Reference"))
  (`self.K2_SetActorLocation` (`KismetMathLibrary.MakeVector` (.x (`self.K2_GetActorLocation` ActivityActor)) (.y (`self.K2_GetActorLocation` ActivityActor)) (.z (`self.K2_GetActorLocation`))))
  (`|PlayMontage` (`self.Mesh`) Montage
    (:`OnCompleted`
      (bind _selectedactivity (`self.SelectedActivity`)
        (:`then`
          (`KismetArrayLibrary.Array_RemoveItem` (`/Game/EasyBuildingSystem/Blueprints/BuildingObjects/Placeable/Poles/BP_EBS_Building_Activity.EmployeesUsing` _selectedactivity) self)
          (`self.GoToJobActivity`))
        (:`else`)))))

(fn `ApplyShapeKeys`
  (params (ShapeKeys :type "Map of String to Float (double-precision)") (Mesh :type "SkeletalMeshComponent Object Reference"))
  (returns (Result :type Boolean))
  (bind _keys (`BlueprintMapLibrary.Map_Keys` ShapeKeys))
  (for _array_element _keys
    (`SkeletalMeshComponent.SetMorphTarget` Mesh (`KismetStringLibrary.Conv_StringToName` _array_element) (`BlueprintMapLibrary.Map_Find` ShapeKeys _array_element) false))
  (return true))

(fn `GetChildMesh`
  (returns (ChildMesh :type "Array of SkeletalMesh Object Reference"))
  (locals (Temp :type "Array of SkeletalMesh Object Reference"))
  (for _array_element (`SceneComponent.GetChildrenComponents` (`self.Mesh`) true)
    (bind _ascomponente_de_malla_del_esqueleto (cast `SkeletalMeshComponent` _array_element))
    (`KismetArrayLibrary.Array_Add` (`local.Temp`) (`SkinnedMeshComponent.SkeletalMesh` _ascomponente_de_malla_del_esqueleto)))
  (return (`local.Temp`)))

(fn `GetJobActivity`
  (returns (Activity :type "/Game/EasyBuildingSystem/Blueprints/BuildingObjects/Placeable/Poles/BP_EBS_Building_Activity Object Reference"))
  (locals (Temp :type "Array of /Game/EasyBuildingSystem/Blueprints/BuildingObjects/Placeable/Poles/BP_EBS_Building_Activity Object Reference"))
  (bind _outitem (`KismetArrayLibrary.Array_Random` (`local.Temp`)))
  (bind _outactors (`GameplayStatics.GetAllActorsOfClass` "/Game/EasyBuildingSystem/Blueprints/BuildingObjects/Placeable/Poles/BP_EBS_Building_Activity.BP_EBS_Building_Activity_C"))
  (for _array_element _outactors
    (if (< (`KismetArrayLibrary.Array_Length` (`/Game/EasyBuildingSystem/Blueprints/BuildingObjects/Placeable/Poles/BP_EBS_Building_Activity.EmployeesUsing` _array_element)) (`/Game/EasyBuildingSystem/Blueprints/BuildingObjects/Placeable/Poles/BP_EBS_Building_Activity.EmployeesMax` _array_element))
      (`KismetArrayLibrary.Array_Add` (`local.Temp`) _array_element)))
  (`/Engine/EditorBlueprintResources/StandardMacros.IsValid` _outitem
    (:`Is Valid`
      (return _outitem))))

(fn `GetLockerRoom`
  (returns (Location :type "Vector Structure"))
  (bind _outactors (`GameplayStatics.GetAllActorsOfClass` "/Game/EasyBuildingSystem/Blueprints/BuildingObjects/Placeable/BP_EBS_Building_Locker_Room.BP_EBS_Building_Locker_Room_C"))
  (bind _outitem (`KismetArrayLibrary.Array_Random` _outactors))
  (`/Engine/EditorBlueprintResources/StandardMacros.IsValid` _outitem
    (:`Is Valid`
      (return (`self.K2_GetActorLocation` _outitem)))
    (:`Is Not Valid`
      (return (0.0 0.0 0.0)))))

(fn `GetOwnEmployeesSlot`
  (returns (Find :type Boolean) (Widget :type "/Game/BurdelKing/WBP_OwnEmployeSlot Object Reference"))
  (bind _foundwidgets (`WidgetBlueprintLibrary.GetAllWidgetsOfClass` "/Game/BurdelKing/WBP_OwnEmployeSlot.WBP_OwnEmployeSlot_C" false))
  (for _array_element _foundwidgets
    (if (== (`/Game/BurdelKing/WBP_OwnEmployeSlot.UniqueID` _array_element) (`self.UniqueID`))
      (return true _array_element)))
  (return false null))

(fn `GetWorkPlace`
  (returns (Location :type "Vector Structure"))
  (bind _outactors (`GameplayStatics.GetAllActorsOfClass` "/Game/EasyBuildingSystem/Blueprints/BuildingObjects/Modular/BP_EBS_Building_Foundation.BP_EBS_Building_Foundation_C"))
  (bind _outitem (`KismetArrayLibrary.Array_Random` _outactors))
  (`/Engine/EditorBlueprintResources/StandardMacros.IsValid` _outitem
    (:`Is Valid`
      (return (`self.K2_GetActorLocation` _outitem)))
    (:`Is Not Valid`
      (return (0.0 0.0 0.0)))))

(fn `SetCloth`
  (returns (Result :type Boolean))
  (bind _mesh (`self.Mesh`))
  (bind (_mesh_2 _materials) (break `/Game/ProceduralGeneration/ClothStruct` (`.Cloth_40_8384C8A04664738C5C65CDBF6B551E65` (break `/Game/ProceduralGeneration/ProceduralCharacterStruct` (`self.CharacterInfo`)))))
  (bind _returnvalue (`AddComponent|NODE_AddSkeletalMeshComponent-0`))
  (`SkinnedMeshComponent.SetSkinnedAssetAndUpdate` _returnvalue _mesh_2 true)
  (`KismetArrayLibrary.Array_Add` (`self.Meshes`) _returnvalue)
  (`SceneComponent.K2_AttachToComponent` _returnvalue _mesh "None" "KeepRelative" "KeepRelative" "KeepRelative" true)
  (`SkinnedMeshComponent.SetLeaderPoseComponent` _returnvalue _mesh false)
  (for (_array_element _array_index) _materials
    (`PrimitiveComponent.SetMaterial` _returnvalue _array_index _array_element))
  (return true))

(fn `SetMeshes`
  (returns (Result :type Boolean))
  (bind _mesh (`self.Mesh`))
  (bind (_uniqueid _shapekey _class _name _facerender _facerenderbytes _rendersize _bodymesh _animationbp) (break `/Game/ProceduralGeneration/ProceduralCharacterStruct` (`self.CharacterInfo`)))
  (`SkinnedMeshComponent.SetSkinnedAssetAndUpdate` _mesh _bodymesh true)
  (`SkeletalMeshComponent.SetAnimInstanceClass` _mesh _animationbp)
  (`KismetArrayLibrary.Array_Add` (`self.Meshes`) (`self.Mesh`))
  (`self.SetCloth`)
  (return true))

(fn `UserConstructionScript`)