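; BP_CarSpawner is a placed actor that spawns BP_EmployeerCar actors or, when flagged as a remover, destroys them.
; Non-removers run a looping timer, its random interval picked once at BeginPlay, spawning cars with the spline and spawner reference unless ForEmployees is set.
; SpawnCarForEmployeer spawns a car on demand for a given employee ID.
; Removers use box overlap to destroy cars whose Spawner is another actor.
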(event `self.ReceiveBeginPlay`
  (if (not (`self.IsRemover`))
    (`KismetSystemLibrary.K2_SetTimerDelegate` (delegate `SpawnCars`) (`KismetMathLibrary.RandomFloatInRange` (`self.SpawnTimeMin`) (`self.SpawnTimeMax`)) true)))

(event `SpawnCars`
  (if (not (`self.ForEmployees?`))
    (bind _returnvalue (`|SpawnActorFromClass` "/Game/Core/EmployeerCar/BP_EmployeerCar.BP_EmployeerCar_C" (`KismetMathLibrary.MakeTransform` (+ (.location (`self.GetTransform`)) (0.0 0.0 25.0)) (.rotation (`self.GetTransform`)) (.scale (`self.GetTransform`))) "AlwaysSpawn" "OverrideRootScale" null null))
    (set `/Game/Vehicles/VehicleBP/Sedan/BP_CarBase.SplineActor` (`self.Spline Actor`) _returnvalue)
    (set `/Game/Core/EmployeerCar/BP_EmployeerCar.Spawner` self _returnvalue)))

(event `SpawnCarForEmployeer`
  (params (UniqueID :type Integer))
  (bind _returnvalue (`|SpawnActorFromClass` "/Game/Core/EmployeerCar/BP_EmployeerCar.BP_EmployeerCar_C" (`KismetMathLibrary.MakeTransform` (+ (.location (`self.GetTransform`)) (0.0 0.0 50.0)) (.rotation (`self.GetTransform`)) (.scale (`self.GetTransform`))) "AlwaysSpawn" "OverrideRootScale" null null))
  (`/Game/Core/EmployeerCar/BP_EmployeerCar.SetCarForEmployeer` _returnvalue UniqueID))

(event `self.Box.OnComponentBeginOverlap`
  (params (OverlappedComponent :type "PrimitiveComponent Object Reference") (OtherActor :type "Actor Object Reference") (OtherComp :type "PrimitiveComponent Object Reference") (OtherBodyIndex :type Integer) (bFromSweep :type Boolean) (SweepResult :type "HitResult Structure (by ref)"))
  (if (`self.IsRemover`)
    (bind _asbp_employeer_car (cast `/Game/Core/EmployeerCar/BP_EmployeerCar` OtherActor))
    (if (!= (`/Game/Core/EmployeerCar/BP_EmployeerCar.Spawner` _asbp_employeer_car) self)
      (`self.K2_DestroyActor` _asbp_employeer_car))))

(fn `UserConstructionScript`)