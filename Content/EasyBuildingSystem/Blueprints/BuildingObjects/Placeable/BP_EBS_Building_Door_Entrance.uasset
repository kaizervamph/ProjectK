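; Placeable club entrance door for the building system that shows open/closed text and switches character lighting as people pass through.
; On build completion it reads ClubOpen from the player controller to set the text, and cursor hover drives HoverFX.
; In and Out trigger boxes turn lighting channel 0 (sun) off or on for employee and pedestrian skeletal meshes.
; Clicking does nothing, as the ClubOpen toggle is unwired.
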(event `self.ReceiveBeginPlay`
  (`parent.ReceiveBeginPlay`))

(event `self.StaticMesh.OnBeginCursorOver`
  (params (TouchedComponent :type "PrimitiveComponent Object Reference"))
  (`self.HoverFX` true))

(event `self.StaticMesh.OnEndCursorOver`
  (params (TouchedComponent :type "PrimitiveComponent Object Reference"))
  (`self.HoverFX` false))

(event `self.StaticMesh.OnClicked`
  (params (TouchedComponent :type "PrimitiveComponent Object Reference") (ButtonPressed :type "Key Structure")))

(event `DoorIndicator`
  (params (Value :type Boolean))
  (`SceneComponent.SetVisibility` (`self.TextRender_Open`) Value false)
  (`SceneComponent.SetVisibility` (`self.TextRender_Close`) (not Value) false)
  (`PrimitiveComponent.SetCollisionResponseToChannel` (`self.StaticMesh`) "ECC_Visibility" "ECR_Block")
  (`PrimitiveComponent.SetCollisionResponseToChannel` (`self.StaticMesh`) "ECC_GameTraceChannel5" "ECR_Block"))

(event `ChangeSunChannel`
  (params (RootComponent :type "Actor Object Reference") (Value :type Boolean))
  (for _array_element (`SceneComponent.GetChildrenComponents` (`Actor.RootComponent` RootComponent) true)
    (bind _ascomponente_de_malla_del_esqueleto (cast `SkeletalMeshComponent` _array_element))
    (`PrimitiveComponent.SetLightingChannels` _ascomponente_de_malla_del_esqueleto Value false true)))

(event `self.Box_In.OnComponentBeginOverlap`
  (params (OverlappedComponent :type "PrimitiveComponent Object Reference") (OtherActor :type "Actor Object Reference") (OtherComp :type "PrimitiveComponent Object Reference") (OtherBodyIndex :type Integer) (bFromSweep :type Boolean) (SweepResult :type "HitResult Structure (by ref)"))
  (bind _asbp_employees_base (cast `/Game/Core/BP_EmployeesBase` OtherActor)
    (:`then`
      (`self.ChangeSunChannel` _asbp_employees_base))
    (:`CastFailed`
      (bind _asbp_pedestrian_base (cast `/Game/Core/Pedestrians/BP_PedestrianBase` OtherActor))
      (`self.ChangeSunChannel` _asbp_pedestrian_base))))

(event `self.Box_Out.OnComponentBeginOverlap`
  (params (OverlappedComponent :type "PrimitiveComponent Object Reference") (OtherActor :type "Actor Object Reference") (OtherComp :type "PrimitiveComponent Object Reference") (OtherBodyIndex :type Integer) (bFromSweep :type Boolean) (SweepResult :type "HitResult Structure (by ref)"))
  (bind _asbp_employees_base (cast `/Game/Core/BP_EmployeesBase` OtherActor)
    (:`then`
      (`self.ChangeSunChannel` _asbp_employees_base true))
    (:`CastFailed`
      (bind _asbp_pedestrian_base (cast `/Game/Core/Pedestrians/BP_PedestrianBase` OtherActor))
      (`self.ChangeSunChannel` _asbp_pedestrian_base true))))

(fn `CompleteBuild`
  (params (PlayerController :type "PlayerController Object Reference"))
  (returns (Success :type Boolean))
  (bind _asbp_ebs_player_controller (cast `/Game/EasyBuildingSystem/Blueprints/Game/BP_EBS_PlayerController` PlayerController)
    (:`then`
      (`self.DoorIndicator` (`/Game/EasyBuildingSystem/Blueprints/Game/BP_EBS_PlayerController.ClubOpen?` _asbp_ebs_player_controller)))
    (:`CastFailed`
      _))
  (bind _success (`parent.CompleteBuild` PlayerController))
  (return _success))

(fn `UserConstructionScript`
  (`parent.UserConstructionScript`))