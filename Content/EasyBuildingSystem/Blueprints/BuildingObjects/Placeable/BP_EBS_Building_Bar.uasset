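; A placeable bar building for the Easy Building System that offers a single socket for users and pays out a resource for activity.
; Construction and ResetActor refill the free-socket list with BarSocket and clear Users, while GetFreeSocket returns the first free socket's world transform.
; PayActivity adds a random whole amount of one resource type to the player controller's ResourcesComponent.
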(event `self.ReceiveTick`
  (params (DeltaSeconds :type "Float (single-precision)")))

(event `PayActivity`
  (bind _asbp_ebs_player_controller (cast `/Game/EasyBuildingSystem/Blueprints/Game/BP_EBS_PlayerController` (`GameplayStatics.GetPlayerController` 0)))
  (`/Game/EasyBuildingSystem/Blueprints/Components/BP_EBS_ResourcesComponent.AddResource` (`/Game/EasyBuildingSystem/Blueprints/Game/BP_EBS_PlayerController.ResourcesComponent` _asbp_ebs_player_controller) (make `/Game/EasyBuildingSystem/Blueprints/Structures/STR_EBS_Resource` "NewEnumerator3" (`KismetMathLibrary.Conv_IntToDouble` (`KismetMathLibrary.FTrunc` (`KismetMathLibrary.RandomFloatInRange` 5.0 15.0))))))

(event `self.ResetActor`
  (`self.SetFreeSockets`)
  (`self.ClearUsers`))

(fn `ClearUsers`
  (returns (Success :type Boolean))
  (`KismetArrayLibrary.Array_Clear` (`self.Users`))
  (return true))

(fn `GetFreeSocket`
  (returns (Location :type "Vector Structure") (Rotation :type "Rotator Structure") (Socket :type "SceneComponent Object Reference") (Find :type Boolean))
  (bind _freesockets (`self.FreeSockets`))
  (bind _output (`|GetArrayItem` _freesockets))
  (if (`KismetArrayLibrary.Array_IsValidIndex` _freesockets)
    (return (`SceneComponent.K2_GetComponentLocation` _output) (`SceneComponent.K2_GetComponentRotation` _output) _output true)
    (else
      (return (0.0 0.0 0.0) (struct) null false))))

(fn `SetFreeSockets`
  (returns (Success :type Boolean))
  (set `self.FreeSockets` (`|MakeArray` (`self.Bar_Socket`)))
  (return true))

(fn `UserConstructionScript`
  (`parent.UserConstructionScript`)
  (`self.SetFreeSockets`)
  (`self.ClearUsers`))