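; PC_CharacterCreator is the player controller for the character creator screen.
; On BeginPlay it creates the WBP_CharacterCreator widget, stores it, sets game-and-UI input focused on it and adds it to the viewport.
; It then finds the first BP_CharacterCreator actor in the level and passes that actor's morph targets to the widget through LoadMorphoTarget.
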(event `self.ReceiveBeginPlay`
  (bind _returnvalue (`|CreateWidget` "/Game/CharacterCreator/WBP_CharacterCreator.WBP_CharacterCreator_C"))
  (set `self.CC` _returnvalue)
  (`WidgetBlueprintLibrary.SetInputMode_GameAndUIEx` self _returnvalue)
  (`UserWidget.AddToViewport` _returnvalue 0)
  (bind _outactors (`GameplayStatics.GetAllActorsOfClass` "/Game/CharacterCreator/BP_CharacterCreator.BP_CharacterCreator_C"))
  (if (`KismetArrayLibrary.Array_IsValidIndex` _outactors)
    (bind _cc (`self.CC`)
      (:`then`
        (`/Game/CharacterCreator/WBP_CharacterCreator.LoadMorphoTarget` _cc (`/Game/CharacterCreator/BP_CharacterCreator.GetMorphoTargets` (`|GetArrayItem` _outactors))))
      (:`else`))))

(fn `UserConstructionScript`)