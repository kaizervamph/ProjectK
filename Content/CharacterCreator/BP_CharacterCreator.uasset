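; Character creator actor that previews a customizable character with morph targets, skin color, clothing and looping animations.
; Hair, Cloth and Shoes follow Body through master pose, and clothing meshes come from DT_Cloth, with colors set as material parameters.
; Child-actor BP_CC_Camera views for head, chest, pelvis and body blend on request, alongside a free pawn view.
; Input rotates Body and Body1, and the mouse wheel zooms the active camera.
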(event `self.ReceiveBeginPlay`
  (`self.ChangeCamera` "Body" 0.0))

(event `Key|MouseScrollDown`
  (params (Key :type "Key Structure"))
  (:`Pressed`
    (`self.ChangeCameraZoom` 5.0)))

(event `Key|MouseScrollUp`
  (params (Key :type "Key Structure"))
  (:`Pressed`
    (`self.ChangeCameraZoom` -5.0)))

(event `RotateCharacter`
  (params (Value :type "Float (double-precision)"))
  (`SceneComponent.K2_AddLocalRotation` (`self.Body`) (`KismetMathLibrary.MakeRotator` 0.0 0.0 Value) false false)
  (`SceneComponent.K2_AddLocalRotation` (`self.Body1`) (`KismetMathLibrary.MakeRotator` 0.0 0.0 Value) false false))

(fn `ChangeAnimation`
  (params (NewAnimToPlay :type "AnimationAsset Object Reference"))
  (returns (Success :type Boolean))
  (`SkeletalMeshComponent.PlayAnimation` (`self.Body`) NewAnimToPlay true)
  (`SkeletalMeshComponent.PlayAnimation` (`self.Body1`) NewAnimToPlay true)
  (return true))

(fn `ChangeCamera`
  (params (Type :type String) (BlendTime :type "Float (double-precision)" :default 1.0))
  (returns (Success :type Boolean))
  (if (`KismetStringLibrary.EqualEqual_StrStr` Type "Free")
    (set `self.CurrentCamera` "Free")
    (set `self.CurrentCameraActor` null)
    (`PlayerController.SetViewTargetWithBlend` (`GameplayStatics.GetPlayerController` 0) (`GameplayStatics.GetPlayerPawn` 0) 0.0 "VTBlend_Linear" 0.0 false)
    (return true)
    (else
      (for _array_element (`self.GetCameras`)
        (bind _type (`/Game/CharacterCreator/BP_CC_Camera.Type` _array_element))
        (if (`KismetStringLibrary.EqualEqual_StrStr` _type Type)
          (set `self.CurrentCamera` _type)
          (set `self.CurrentCameraActor` _array_element)
          (`/Game/CharacterCreator/BP_CC_Camera.ResetArmPosition` _array_element)
          (`PlayerController.SetViewTargetWithBlend` (`GameplayStatics.GetPlayerController` 0) _array_element BlendTime "VTBlend_Linear" 0.0 true)
          (return true)))
      (return false))))

(fn `ChangeCameraZoom`
  (params (Value :type "Float (double-precision)"))
  (returns (Success :type Boolean))
  (if (`KismetStringLibrary.NotEqual_StrStr` (`self.CurrentCamera`) "Free")
    (for _array_element (`self.GetCameras`)
      (if (`KismetStringLibrary.EqualEqual_StrStr` (`/Game/CharacterCreator/BP_CC_Camera.Type` _array_element) (`self.CurrentCamera`))
        (`/Game/CharacterCreator/BP_CC_Camera.CameraZoom` _array_element Value)
        (return true)))
    (else
      (return false))))

(fn `ChangeCloth`
  (params (ClothType :type "/Game/ProceduralGeneration/ClothTypesEnum Enum" :default "NewEnumerator0") (ClothRowName :type Name))
  (returns (Success :type Boolean))
  (bind _returnvalue (`|GetDataTableRow` "/Game/ProceduralGeneration/DT_Cloth.DT_Cloth" ClothRowName)
    (:`then`
      (`SkinnedMeshComponent.SetSkinnedAssetAndUpdate` (select `/Game/ProceduralGeneration/ClothTypesEnum` ClothType :`NewEnumerator0` (`self.Shoes`) :`NewEnumerator1` (`self.Cloth`)) (`.Mesh_3_DEFE4D3745732CB64F5ED38AADFC0985` (break `/Game/ProceduralGeneration/ClothStruct` _returnvalue)) false)
      (return true))
    (:`RowNotFound`
      (return false))))

(fn `ChangeClothColor`
  (params (Color :type "LinearColor Structure") (ClothType :type "/Game/ProceduralGeneration/ClothTypesEnum Enum" :default "NewEnumerator0"))
  (returns (Success :type Boolean))
  (`MeshComponent.SetVectorParameterValueOnMaterials` (select `/Game/ProceduralGeneration/ClothTypesEnum` ClothType :`NewEnumerator0` (`self.Shoes`) :`NewEnumerator1` (`self.Cloth`) :!type "MeshComponent Object Reference") "Color" (`KismetMathLibrary.Conv_LinearColorToVector` Color))
  (return true))

(fn `ChangePoleVisibility`
  (params (Value :type Boolean))
  (returns (Success :type Boolean))
  (`SceneComponent.SetVisibility` (`self.Pole_Base_Visor`) Value false)
  (return true))

(fn `ChangeSkinColor`
  (params (Color :type "LinearColor Structure"))
  (returns (Success :type Boolean))
  (`MeshComponent.SetVectorParameterValueOnMaterials` (`self.Body`) "SkinColor" (`KismetMathLibrary.Conv_LinearColorToVector` Color))
  (return true))

(fn `ClearAllMorphoTargets`
  (returns (Success :type Boolean))
  (`SkeletalMeshComponent.ClearMorphTargets` (`self.Body`))
  (return true))

(fn `GetCameras`
  (returns (Cameras :type "Array of /Game/CharacterCreator/BP_CC_Camera Object Reference"))
  (return (`|MakeArray` (cast `/Game/CharacterCreator/BP_CC_Camera` (`ChildActorComponent.ChildActor` (`self.ChildActor_Head`)) :!pure true) (cast `/Game/CharacterCreator/BP_CC_Camera` (`ChildActorComponent.ChildActor` (`self.ChildActor_Chest`)) :!pure true) (cast `/Game/CharacterCreator/BP_CC_Camera` (`ChildActorComponent.ChildActor` (`self.ChildActor_Pelvis`)) :!pure true) (cast `/Game/CharacterCreator/BP_CC_Camera` (`ChildActorComponent.ChildActor` (`self.ChildActor_Body`)) :!pure true))))

(fn `GetMorphoTarget`
  (params (MorphTargetName :type Name))
  (returns (ReturnValue :type "Float (double-precision)"))
  (return (`SkeletalMeshComponent.GetMorphTarget` (`self.Body`) MorphTargetName)))

(fn `GetMorphoTargets`
  (returns (MorphoTargets :type "Array of String"))
  (return (`SkeletalMesh.K2_GetAllMorphTargetNames` (`SkinnedMeshComponent.SkeletalMesh` (`self.Body`)))))

(fn `SetMorphoTarget`
  (params (MorphTargetName :type Name) (Value :type "Float (double-precision)"))
  (returns (Success :type Boolean))
  (`SkeletalMeshComponent.SetMorphTarget` (`self.Body`) MorphTargetName Value true)
  (return true))

(fn `UserConstructionScript`
  (`SkinnedMeshComponent.SetLeaderPoseComponent` (`self.Hair`) (`self.Body`) false)
  (`SkinnedMeshComponent.SetLeaderPoseComponent` (`self.Cloth`) (`self.Body`) false)
  (`SkinnedMeshComponent.SetLeaderPoseComponent` (`self.Shoes`) (`self.Body`) false))