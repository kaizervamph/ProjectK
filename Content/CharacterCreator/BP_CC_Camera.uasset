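; BP_CC_Camera is a spring-arm camera actor for the character creator, driven by zoom and rotate events.
; CameraZoom offsets the arm length only when the result stays within ZoomMin and ZoomMax, rejecting out-of-range steps rather than clamping them.
; RotateCamera adds local yaw to the arm.
; Construction sets the default length from LongitudDelBrazoDeDestino, and ResetArmPosition restores it along with zero relative rotation.
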(event `CameraZoom`
  (params (Value :type "Float (double-precision)"))
  (if (`KismetMathLibrary.InRange_FloatFloat` (+ (`SpringArmComponent.TargetArmLength` (`self.SpringArm`)) Value) (`self.ZoomMin`) (`self.ZoomMax`))
    (set `SpringArmComponent.TargetArmLength` (+ (`SpringArmComponent.TargetArmLength` (`self.SpringArm`)) Value) (`self.SpringArm`))))

(event `RotateCamera`
  (params (`Z (Yaw)` :type "Float (double-precision)"))
  (`SceneComponent.K2_AddLocalRotation` (`self.SpringArm`) (`KismetMathLibrary.MakeRotator` 0.0 0.0 `Z (Yaw)`) false false))

(fn `ResetArmPosition`
  (returns (Success :type Boolean))
  (set `SpringArmComponent.TargetArmLength` (`self.Longitud Del Brazo De Destino`) (`self.SpringArm`))
  (`SceneComponent.K2_SetRelativeRotation` :`self` (`self.SpringArm`))
  (return true))

(fn `UserConstructionScript`
  (set `SpringArmComponent.TargetArmLength` (`self.Longitud Del Brazo De Destino`) (`self.SpringArm`)))