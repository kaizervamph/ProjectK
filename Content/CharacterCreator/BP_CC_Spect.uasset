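; BP_CC_Spect is the player-controlled spectator-style pawn for the character creator.
; On BeginPlay it caches the first BP_CharacterCreator in the level, and all input depends on that reference.
; While the creator has a current camera actor, horizontal mouse input rotates the character and other look and movement input is ignored.
; Without one, the mouse turns the view and the axis inputs fly the pawn freely.
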(event `self.ReceiveBeginPlay`
  (bind _outactors (`GameplayStatics.GetAllActorsOfClass` "/Game/CharacterCreator/BP_CharacterCreator.BP_CharacterCreator_C"))
  (if (`KismetArrayLibrary.Array_IsValidIndex` _outactors)
    (set `self.CC` (`|GetArrayItem` _outactors))))

(event `InputAxisKey|MouseX`
  (params (AxisValue :type "Float (single-precision)"))
  (bind _cc (`self.CC`)
    (:`then`
      (bind _currentcameraactor (`/Game/CharacterCreator/BP_CharacterCreator.CurrentCameraActor` _cc)
        (:`then`
          (bind _result (`/Engine/EditorBlueprintResources/StandardMacros.NegateFloat` AxisValue)
            (:`  `
              (`/Game/CharacterCreator/BP_CharacterCreator.RotateCharacter` _cc _result))))
        (:`else`
          (`self.AddControllerYawInput` AxisValue))))
    (:`else`)))

(event `InputAxisKey|MouseY`
  (params (AxisValue :type "Float (single-precision)"))
  (bind _cc (`self.CC`)
    (:`then`
      (`/Game/CharacterCreator/BP_CharacterCreator.CurrentCameraActor` _cc
        (:`then`)
        (:`else`
          (bind _result (`/Engine/EditorBlueprintResources/StandardMacros.NegateFloat` AxisValue)
            (:`  `
              (`self.AddControllerPitchInput` _result))))))
    (:`else`)))

(event `InputAxis|MoveForward`
  (params (AxisValue :type "Float (single-precision)"))
  (bind _cc (`self.CC`)
    (:`then`
      (`/Game/CharacterCreator/BP_CharacterCreator.CurrentCameraActor` _cc
        (:`then`)
        (:`else`
          (`self.MoveForward` AxisValue))))
    (:`else`)))

(event `InputAxis|MoveRight`
  (params (AxisValue :type "Float (single-precision)"))
  (bind _cc (`self.CC`)
    (:`then`
      (`/Game/CharacterCreator/BP_CharacterCreator.CurrentCameraActor` _cc
        (:`then`)
        (:`else`
          (`self.MoveRight` AxisValue))))
    (:`else`)))

(fn `UserConstructionScript`)