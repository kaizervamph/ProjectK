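; Actor that procedurally generates random female employee attributes and serves as a captured 3D preview of a character.
; Outside the CharacterCreator level, BeginPlay sends the generated batch to BP_DollRenderActor for rendering; finished characters are stored by name.
; Loading a character builds tagged cloth and hair meshes, then maps averaged needs stats onto facial morph targets.
; Its scene capture shows only itself, with toggleable mouse-driven body rotation.
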(event `self.ReceiveBeginPlay`
  (`|ExecutionSequence`
    (:`then_0`
      (bind _returnvalue (`GameplayStatics.GetCurrentLevelName` true))
      (if (`KismetStringLibrary.NotEqual_StrStr` _returnvalue "CharacterCreator")
        (bind _generatedcharacters (`self.GenerateEmployees` (`self.Amount`)))
        (bind (_find _actor) (`self.GetRenderActor`))
        (if _find
          (`/Game/Core/BP_DollRenderActor.GenerateRendersFromAttributes` _actor _generatedcharacters)
          (else
            (`KismetSystemLibrary.PrintString` "No Render Actor In Level" true true (struct :`R` 1.0 :`G` 0.020833 :`B` 0.020833 :`A` 1.0) 20.0)))))
    (:`then_1`
      (`KismetArrayLibrary.Array_Add` (`SceneCaptureComponent.ShowOnlyActors` (`self.SceneCaptureComponent2D`)) self))
    (:`then_2`
      (`self.UseActor` false))))

(event `AddGeneratedCharacter`
  (params (Character :type "/Game/ProceduralGeneration/ProceduralCharacterStruct Structure") (RenderActor :type "/Game/Core/BP_DollRenderActor Object Reference"))
  (`BlueprintMapLibrary.Map_Add` (`self.GeneratedCharacters`) (`.Name_17_AD6AB613456DD9AD1C8A2F854253C0B0` (break `/Game/ProceduralGeneration/ProceduralCharacterStruct` Character)) Character)
  (`/Game/Core/BP_DollRenderActor.ResetCapture` RenderActor))

(event `LoadCharacterForVisualize`
  (params (CharacterInfo :type "/Game/ProceduralGeneration/ProceduralCharacterStruct Structure"))
  (bind ((`ShapeKey_4_ECC249F94D380943E297EBA44B13C32A` _shapekey) (`Cloths_53_8384C8A04664738C5C65CDBF6B551E65` _cloths) (`Statistics_45_B418B5FE4C0DD41AAC69AD9EE1648F94` _statistics)) (break `/Game/ProceduralGeneration/ProceduralCharacterStruct` CharacterInfo))
  (`self.AddClothMeshes` _cloths CharacterInfo)
  (bind _value (`self.DeductHappiness` _statistics))
  (`self.ExpressionUpdate` (`KismetMathLibrary.MapRangeUnclamped` (/ _value 100.0) 0.0 1.0 -1.0 1.0) _shapekey))

(event `ExpressionUpdate`
  (params (Value :type "Float (double-precision)") (ShapeKeys :type "Map of String to Float (double-precision)"))
  (bind _expressions (`/Game/ProceduralGeneration/FL_ProceduralGeneration.GetFemaleExpressionShapeKeys` ShapeKeys))
  (bind _keys (`BlueprintMapLibrary.Map_Keys` _expressions))
  (for _array_element _keys
    (`SkeletalMeshComponent.SetMorphTarget` (`self.BodyMesh`) (`KismetStringLibrary.Conv_StringToName` _array_element) Value true)))

(event `SetMaterialBody`
  (`/Game/ProceduralGeneration/FL_ProceduralGeneration.SetBodyMesh` (make `/Game/ProceduralGeneration/ProceduralCharacterStruct` :`BodyMesh` "/Game/Assets/Female/SK_Female_01.SK_Female_01" :`AnimationBP` "/Game/Assets/Female/ABP_Female_01.ABP_Female_01_C" :`SkinColor` (struct :`A` 1.0)) (`self.BodyMesh`)))

(event `InputAxisKey|MouseX`
  (params (AxisValue :type "Float (single-precision)"))
  (bind _result (`/Engine/EditorBlueprintResources/StandardMacros.NegateFloat` (* AxisValue 5.0))
    (:`  `
      (`SceneComponent.K2_AddLocalRotation` (`self.BodyMesh`) (`KismetMathLibrary.MakeRotator` 0.0 0.0 _result) false false))))

(event `InputAxisKey|MouseY`
  (params (AxisValue :type "Float (single-precision)")))

(event `UseActor`
  (params (Value :type Boolean))
  (bind _returnvalue (`GameplayStatics.GetPlayerController` 0))
  (if Value
    (`self.EnableInput` _returnvalue)
    (else
      (`self.DisableInput` _returnvalue))))

(fn `AddClothMeshes`
  (params (Cloths :type "Array of /Game/ProceduralGeneration/ClothStruct Structure") (CharacterInfo :type "/Game/ProceduralGeneration/ProceduralCharacterStruct Structure (by ref)"))
  (returns (HairComponent :type "SkeletalMeshComponent Object Reference"))
  (locals (ClothsTemp :type "Array of SkeletalMeshComponent Object Reference") (MeshesTemp :type "Array of SkeletalMeshComponent Object Reference"))
  (for _array_element Cloths
    (bind _returnvalue (`AddComponent|NODE_AddSkeletalMeshComponent-3`))
    (`KismetArrayLibrary.Array_Add` (`ActorComponent.ComponentTags` _returnvalue) (`KismetStringLibrary.Conv_StringToName` (`|GetEnumeratorNameAsString` (`.Type_11_19E0FABA49E91A75A4CFFF89C012AE1B` (break `/Game/ProceduralGeneration/ClothStruct` _array_element)))))
    (`KismetArrayLibrary.Array_Add` (`local.ClothsTemp`) _returnvalue)
    (`KismetArrayLibrary.Array_Add` (`local.MeshesTemp`) _returnvalue))
  (bind _returnvalue_2 (`AddComponent|NODE_AddSkeletalMeshComponent-4`))
  (`KismetArrayLibrary.Array_Add` (`ActorComponent.ComponentTags` _returnvalue_2) "Hair")
  (`KismetArrayLibrary.Array_Add` (`local.MeshesTemp`) _returnvalue_2)
  (`/Game/ProceduralGeneration/FL_ProceduralGeneration.ConfigCharacterMeshes` self (`self.BodyMesh`) (`local.MeshesTemp`) CharacterInfo (`local.ClothsTemp`) _returnvalue_2 Cloths)
  (return _returnvalue_2))

(fn `DeductHappiness`
  (params (Statistics :type "Map of String to Float (double-precision)"))
  (returns (Value :type "Float (double-precision)"))
  (return (/ (+ (`BlueprintMapLibrary.Map_Find` Statistics "Energy") (`BlueprintMapLibrary.Map_Find` Statistics "Hunger") (`BlueprintMapLibrary.Map_Find` Statistics "Thirst") (`BlueprintMapLibrary.Map_Find` Statistics "Bath")) 4.0)))

(fn `GenerateEmployees`
  (params (Amount :type Integer))
  (returns (GeneratedCharacters :type "Array of /Game/ProceduralGeneration/ProceduralCharacterStruct Structure"))
  (locals (Temp :type "Array of /Game/ProceduralGeneration/ProceduralCharacterStruct Structure"))
  (for _index (range 1 (+ Amount 1))
    (bind (_attributes _nameused) (`/Game/ProceduralGeneration/FL_ProceduralGeneration.GenerateRandomFemaleInfo` (`self.GeneratedNames`) _index))
    (`KismetArrayLibrary.Array_Add` (`self.GeneratedNames`) _nameused)
    (`KismetArrayLibrary.Array_Add` (`local.Temp`) _attributes))
  (return (`local.Temp`)))

(fn `GetNamesFromGenerated`
  (params (GeneratedCharacters :type "Map of String to /Game/ProceduralGeneration/ProceduralCharacterStruct Structure"))
  (returns (Names :type "Array of String"))
  (bind _keys (`BlueprintMapLibrary.Map_Keys` GeneratedCharacters))
  (return _keys))

(fn `GetRenderActor`
  (returns (Find :type Boolean) (Actor :type "/Game/Core/BP_DollRenderActor Object Reference"))
  (bind _outactors (`GameplayStatics.GetAllActorsOfClass` "/Game/Core/BP_DollRenderActor.BP_DollRenderActor_C"))
  (if (`KismetArrayLibrary.Array_IsValidIndex` _outactors)
    (return true (`|GetArrayItem` _outactors))
    (else
      (return false null))))

(fn `UserConstructionScript`)